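; Moon actor that fades in and lights up at night and fades out when night ends, driven by a ShowMoon event.
; A timeline raises the opacity of a dynamic translucent material, then swaps in a solid material and starts a second timeline that ramps four point lights.
; Hiding reverses the sequence: the lights dim first, then the translucent material returns and fades out.
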(event Custom|ShowMoon
  (params (Night? :type Boolean))
  ;[0.08205 0.03103 1] Show and hide moon at sunset or sunrise
  (bind _output_get (Variables|Default|SetNight? Night?))
  (if _output_get
    (bind _alpha (Timeline|MoonOpacity PlayFromStart)
      (:Update
        (Rendering|Material|SetScalarParameterValue (Variables|Default|GetMoonTranslucentMat) "Opacity" (Math|Float|Lerp 0.0 1.0 _alpha) :!class /Script/Engine.MaterialInstanceDynamic))
      (:Finished
        (if (Variables|Default|GetNight?)
          (bind _returnvalue (Rendering|Material|CreateDynamicMaterialInstance "/Game/ThirdParty/Assets/Moon/M_MoonSolid.M_MoonSolid" "None" "None" :!class /Script/Engine.KismetMaterialLibrary))
          (bind _output_get_2 (Variables|Default|SetMoonSolidMat _returnvalue))
          (Rendering|Material|SetMaterial (Variables|Debug|GetStaticMeshComponent) 0 _output_get_2)
          (bind _alpha_2 (Timeline|LightsOn PlayFromStart)
            (:Update
              (Rendering|Components|Light|SetIntensity (Variables|Default|GetPointLight1) (Math|Float|Lerp 0.0 2e+05 _alpha_2)))
            (:Finished
              (if (not (Variables|Default|GetNight?))
                (Rendering|Material|SetMaterial (Variables|Debug|GetStaticMeshComponent) 0 (Variables|Default|GetMoonTranslucentMat))
                (Timeline|MoonOpacity ReverseFromEnd)))))))
    (else
      (Timeline|LightsOn ReverseFromEnd))))

(event EventBeginPlay
  ;[0.5781 0.5781 0.5781] Moon material set up
  (bind _returnvalue (Rendering|Material|CreateDynamicMaterialInstance "/Game/ThirdParty/Assets/Moon/M_MoonTranslucent.M_MoonTranslucent" "None" "None" :!class /Script/Engine.KismetMaterialLibrary))
  (bind _output_get (Variables|Default|SetMoonTranslucentMat _returnvalue))
  (Rendering|Material|SetScalarParameterValue _output_get "Opacity" 0.0 :!class /Script/Engine.MaterialInstanceDynamic)
  (Rendering|Material|SetMaterial (Variables|Debug|GetStaticMeshComponent) 0 (Variables|Default|GetMoonTranslucentMat)))

(fn ConstructionScript)