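; Campfire Blueprint that switches its flames and firelight on or off through a SpawnFlames event.
; The Spawn flag begins or ends trails on the Flames component and plays or reverses the CampfireIlumination timeline.
; The timeline's alpha lerps the PointLight intensity, so the light ramps up and down with the fire.
; A 2D sound fade-in and fade-out branch exists but is unconnected, so it never runs.
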(event Custom|SpawnFlames
  (params (Spawn? :type Boolean))
  (bind _flames (Variables|Default|GetFlames))
  ;[1 0.2181 0.05805] Spawn flames from campfire
  (if Spawn?
    (Effects|Particles|Trails|BeginTrails _flames "None" "None" "ETrailWidthMode_FromCentre" 0.0)
    (bind _alpha (Timeline|CampfireIlumination PlayFromStart)
      (:Update
        (Rendering|Components|Light|SetIntensity (Variables|Default|GetPointLight) (Math|Float|Lerp 0.0 2.5e+03 _alpha))))
    (else
      (Effects|Particles|Trails|EndTrails _flames)
      (Timeline|CampfireIlumination ReverseFromEnd))))

(fn ConstructionScript)