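; MusicManager plays looping-style 2D ambience for the game and swaps it between a peaceful day track and a night track.
; BeginPlay spawns the day ambience and fades it in.
; The SwitchAmbienceSound event takes a Day flag, fades out the opposite track, then spawns and fades in the new one at reduced volume.
; A delay slightly shorter than the fade-out overlaps the two tracks for a brief crossfade.
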(event Custom|SwitchAmbienceSound
  (params (Day? :type Boolean))
  ;[1 0.1562 0.1562] Switch ambience sounds between day and night
  (if Day?
    (Audio|Components|Audio|FadeOut (Variables|Default|GetNightAmbienceSound) 3.0 0.0 "Linear" :!class /Script/Engine.AudioComponent)
    (Utilities|FlowControl|Delay 2.5)
    (bind _returnvalue (Audio|SpawnSound2D "/Game/Audio/AmbiencePeaceful.AmbiencePeaceful" 0.5 1.0 0.0 0))
    (bind _output_get (Variables|Default|SetDayAmbienceSound _returnvalue))
    (Audio|Components|Audio|FadeIn _output_get 1.0 1.0 0.0 "Linear" :!class /Script/Engine.AudioComponent)
    (else
      (Audio|Components|Audio|FadeOut (Variables|Default|GetDayAmbienceSound) 3.0 0.0 "Linear" :!class /Script/Engine.AudioComponent)
      (Utilities|FlowControl|Delay 2.5)
      (bind _returnvalue_2 (Audio|SpawnSound2D "/Game/Audio/AmbienceNight.AmbienceNight" 0.5 1.0 0.0 0))
      (bind _output_get_2 (Variables|Default|SetNightAmbienceSound _returnvalue_2))
      (Audio|Components|Audio|FadeIn _output_get_2 1.0 1.0 0.0 "Linear" :!class /Script/Engine.AudioComponent))))

(event EventBeginPlay
  ;[0.6912 0.1027 1] Plays day ambience sound at the beginning
  (bind _returnvalue (Audio|SpawnSound2D "/Game/Audio/AmbiencePeaceful.AmbiencePeaceful" 0.5 1.0 0.0 0))
  (bind _output_get (Variables|Default|SetDayAmbienceSound _returnvalue))
  (Audio|Components|Audio|FadeIn _output_get 2.0 1.0 0.0 "Linear" :!class /Script/Engine.AudioComponent))

(fn ConstructionScript)